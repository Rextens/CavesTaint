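; ChunkBP is a map chunk actor whose only working logic is a debug event, with empty construction, BeginPlay and Tick.
; ForTests spawns a TextRenderActor at the given grid coordinates, scaled to 100-unit cells, and displays the passed value.
; Disconnected construction-script nodes remain from voxel generation: a 64-cubed loop, world-offset 3D simplex noise, a threshold check and instanced static mesh placement, none of which run.
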(event `self.ReceiveBeginPlay`)

(event `self.ReceiveTick`
  (params (DeltaSeconds :type "Float (single-precision)")))

(event `self.forTests`
  (params (x :type "Float (single-precision)") (y :type "Float (single-precision)") (z :type "Float (single-precision)") (value :type "Float (single-precision)"))
  (bind _returnvalue (`|SpawnActorFromClass` "/Script/Engine.TextRenderActor" (`KismetMathLibrary.MakeTransform` (* (`KismetMathLibrary.MakeVector` x y z) 100.0)) "Undefined" "OverrideRootScale" null null))
  (`TextRenderComponent.K2_SetText` (`TextRenderActor.TextRender` _returnvalue) (`KismetTextLibrary.Conv_DoubleToText` value "HalfToEven")))

(fn `UserConstructionScript`)