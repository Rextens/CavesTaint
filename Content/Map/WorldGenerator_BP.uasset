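; WorldGenerator_BP is a world generator actor that tracks which chunk the player character occupies.
; Every Tick, it divides the referenced character's location by ChunkSize and floors each axis to store CurrentChunkPosition in chunk-grid coordinates.
; It then calls GetCurrentChunk, whose body is not included here.
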(event `self.ReceiveTick`
  (params (DeltaSeconds :type "Float (single-precision)"))
  (`self.updatePlayerToChunkPosition`)
  (`self.getCurrentChunk`))

(fn `updatePlayerToChunkPosition`
  (bind (_returnvalue_x _returnvalue_y _returnvalue_z) (`KismetMathLibrary.BreakVector` (/ (`self.K2_GetActorLocation` (`self.characterReference`)) (`self.chunkSize`))))
  (set `self.currentChunkPosition` (`KismetMathLibrary.Conv_IntVectorToVector` (make `IntVector` (`KismetMathLibrary.FFloor` _returnvalue_x) (`KismetMathLibrary.FFloor` _returnvalue_y) (`KismetMathLibrary.FFloor` _returnvalue_z)))))

(fn `UserConstructionScript`)