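; Player character that digs terrain and walks with gravity aligned to the surface underfoot.
; Tick points the GravityMovementComponent's gravity against the current floor normal.
; G sphere-traces from the camera to carve and smooth VoxelWorld hits, while C line-traces via LookAt to call Dig on a ChunkBP.
; Equipment widget toggle, teleport, side-stick trace and sphere-overlap destruction are unconnected leftovers.
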(event `self.ReceiveBeginPlay`)

(event `Key|G`
  (params (Key :type "Key Structure"))
  (bind _camera (`self.Camera`))
  (bind _returnvalue (`SceneComponent.K2_GetComponentLocation` _camera))
  (:`Pressed`
    (bind _outhits (`KismetSystemLibrary.SphereTraceMulti` :`Start` _returnvalue :`End` (+ _returnvalue (* (`KismetMathLibrary.GetForwardVector` (`SceneComponent.K2_GetComponentRotation` _camera)) 1000)) :`Radius` 10.0 :`TraceChannel` "TraceTypeQuery1" :`DrawDebugType` "Persistent"))
    (for _array_element _outhits
      (bind _asvoxel_world (cast `VoxelWorld` (`.HitActor` (`GameplayStatics.BreakHitResult` _array_element))))
      (`VoxelSphereTools.RemoveSphere` _asvoxel_world (`.ImpactPoint` (`GameplayStatics.BreakHitResult` _array_element)) 100.0)
      (`VoxelSphereTools.SmoothSphere` _asvoxel_world (`.ImpactPoint` (`GameplayStatics.BreakHitResult` _array_element)) 200.0 0.5))))

(event `self.ReceiveTick`
  (params (DeltaSeconds :type "Float (single-precision)"))
  (bind _charactermovement (`self.CharacterMovement`))
  (bind _asgravity_movement_component (cast `GravityMovementComponent` _charactermovement)
    (:`then`
      (`GravityMovementComponent.SetGravityDirection` _asgravity_movement_component (* (`.Normal` (`GameplayStatics.BreakHitResult` (`.HitResult` (break `FindFloorResult` (`CharacterMovementComponent.CurrentFloor` _charactermovement))))) -1.0)))
    (:`CastFailed`
      (`KismetSystemLibrary.PrintString` "fail"))))

(event `OnBoundsUpdated`
  (params (World :type "VoxelWorld Object Reference") (Bounds :type "IntBox Structure")))

(event `Key|C`
  (params (Key :type "Key Structure"))
  (:`Pressed`
    (`self.lookAt`)))

(event `Key|E`
  (params (Key :type "Key Structure")))

(fn `destroyInTheSphere`
  (bind _returnvalue (`GameplayStatics.GetPlayerCameraManager` 0))
  (bind _newvar_0 (`self.NewVar_0`))
  (bind _returnvalue_2 (`self.K2_GetActorLocation` _returnvalue))
  (bind _outhit (`KismetSystemLibrary.LineTraceSingleForObjects` :`Start` _returnvalue_2 :`End` (+ _returnvalue_2 (* (`self.GetActorForwardVector` _returnvalue) 2000.0)) :`ObjectTypes` _newvar_0 :`DrawDebugType` "ForDuration" :`TraceColor` (struct :`R` 0.934123 :`G` 1.0 :`B` 0.930123 :`A` 1.0)))
  (`KismetSystemLibrary.SphereOverlapActors` (`.Location` (`GameplayStatics.BreakHitResult` _outhit)) 100.0 _newvar_0))

(fn `isStickToTheSide`
  (bind _camera (`self.Camera`))
  (bind _returnvalue (`SceneComponent.K2_GetComponentLocation` _camera))
  (`KismetSystemLibrary.LineTraceSingleForObjects` :`Start` _returnvalue :`End` (+ _returnvalue (* (`SceneComponent.GetForwardVector` _camera) 100.0)) :`ObjectTypes` (`self.NewVar_1`) :`DrawDebugType` "ForDuration"))

(fn `lookAt`
  (bind _returnvalue (`GameplayStatics.GetPlayerCameraManager` 0))
  (bind _returnvalue_2 (`self.K2_GetActorLocation` _returnvalue))
  (bind _outhit (`KismetSystemLibrary.LineTraceSingleForObjects` :`Start` _returnvalue_2 :`End` (+ _returnvalue_2 (* (`self.GetActorForwardVector` _returnvalue) 2000.0)) :`ObjectTypes` (`self.NewVar_0`) :`DrawDebugType` "ForOneFrame" :`TraceColor` (struct :`R` 0.934123 :`G` 1.0 :`B` 0.930123 :`A` 1.0)))
  (bind (_bblockinghit _binitialoverlap _time _distance _location _impactpoint _normal _impactnormal _physmat _hitactor) (`GameplayStatics.BreakHitResult` _outhit))
  (bind _aschunk_bp (cast `/Game/Map/ChunkBP` _hitactor))
  (`Chunk.dig` _aschunk_bp (`self.K2_GetActorLocation` _aschunk_bp) _location))

(fn `UserConstructionScript`)