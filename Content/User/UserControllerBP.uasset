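; User-side Blueprint for a voxel world that spawns a 3D grid of ChunkBP actors around its own location.
; Initialize derives chunk size from voxel size and elements per line, and UpdatePosition converts actor location into chunk coordinates, returning true either way.
; AddChunk spawns missing chunks in a 5x5x5 block around those coordinates, recording them without removal.
; BeginPlay and Tick are empty, so nothing here calls these functions.
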(event `self.ReceiveBeginPlay`)

(event `self.ReceiveTick`
  (params (DeltaSeconds :type "Float (single-precision)")))

(fn `addChunk`
  (bind _chunkcords (`self.chunkCords`))
  (bind _returnvalue (`KismetMathLibrary.Conv_IntToDouble` (`self.chunkSize`)))
  (for _index (range -2 3)
    (for _index_2 (range -2 3)
      (for _index_3 (range -2 3)
        (bind _returnvalue_2 (+ _index (`self.chunkX`)))
        (bind _returnvalue_3 (`KismetMathLibrary.Conv_IntToDouble` _returnvalue_2))
        (bind _returnvalue_4 (+ _index_2 (`self.chunkY`)))
        (bind _returnvalue_5 (`KismetMathLibrary.Conv_IntToDouble` _returnvalue_4))
        (bind _returnvalue_6 (+ _index_3 (`self.chunkZ`)))
        (bind _returnvalue_7 (`KismetMathLibrary.Conv_IntToDouble` _returnvalue_6))
        (if (not (`KismetArrayLibrary.Array_Contains` _chunkcords (`KismetMathLibrary.MakeVector` _returnvalue_3 _returnvalue_5 _returnvalue_7)))
          (`KismetArrayLibrary.Array_Add` _chunkcords (`KismetMathLibrary.MakeVector` _returnvalue_3 _returnvalue_5 _returnvalue_7))
          (bind _returnvalue_8 (`|SpawnActorFromClass` "/Game/Map/ChunkBP.ChunkBP_C" (`KismetMathLibrary.Conv_VectorToTransform` (`KismetMathLibrary.MakeVector` (* _returnvalue_2 _returnvalue) (* _returnvalue_4 _returnvalue) (* _returnvalue_6 _returnvalue))) "Undefined" "OverrideRootScale" null null))
          (`KismetArrayLibrary.Array_Add` (`self.chunks`) _returnvalue_8))))))

(fn `initialize`
  (bind _output_get (set `self.chunkSize` (* (`self.chunkLineElements`) (`self.voxelSize`))))
  (set `self.chunkSizeHalf` (/ _output_get 1)))

(fn `updatePosition`
  (returns (wasChanged :type Boolean))
  (bind _returnvalue (`KismetMathLibrary.Conv_IntToDouble` (`self.chunkSizeHalf`)))
  (bind _output_get (set `self.characterPosition` (`self.K2_GetActorLocation`)))
  (bind _returnvalue_2 (`KismetMathLibrary.FFloor` (/ (.x _output_get) _returnvalue)))
  (bind _returnvalue_3 (`KismetMathLibrary.FFloor` (/ (.y _output_get) _returnvalue)))
  (bind _returnvalue_4 (`KismetMathLibrary.FFloor` (/ (.z _output_get) _returnvalue)))
  (if (or (!= (`self.chunkX`) _returnvalue_2) (!= _returnvalue_3 (`self.chunkY`)) (!= _returnvalue_4 (`self.chunkZ`)))
    (set `self.chunkX` _returnvalue_2)
    (set `self.chunkY` _returnvalue_3)
    (set `self.chunkZ` _returnvalue_4)
    (return true)
    (else
      (return true))))

(fn `UserConstructionScript`)